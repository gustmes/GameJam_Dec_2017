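; Game mode that keeps enemies spawning near the player, up to a maximum count.
; On begin play it resets the TremzinhoDaAlegria friends array to just the player pawn and caches all EnemySpawnPoint locations.
; A looping timer checks the Enemy_BP count, then after a further delay spawns one at the spawn point closest to the player and calls its ChaseActor.
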(event `self.ReceiveBeginPlay`
  (bind _tremzinhodaalegria (`self.TremzinhoDaAlegria`))
  ;[1 1 1] Add Player to array of friends
  (`KismetArrayLibrary.Array_Clear` _tremzinhodaalegria)
  (`KismetArrayLibrary.Array_Add` _tremzinhodaalegria (`GameplayStatics.GetPlayerPawn` 0))
  ;[1 1 1] Make array containing the position of all Enemy Spawn Points
  (bind _outactors (`GameplayStatics.GetAllActorsOfClass` "/Game/Blueprints/EnemySpawnPoint.EnemySpawnPoint_C"))
  (for _array_element _outactors
    (`KismetArrayLibrary.Array_Add` (`self.SpawnPoints`) (`self.K2_GetActorLocation` _array_element)))
  (bind _returnvalue (`KismetSystemLibrary.K2_SetTimerDelegate` (delegate `Spawn Enemy At Closest Spawning Point`) (`self.EnemySpawnDelay`) true))
  (set `self.Timer` _returnvalue))

(event `Spawn Enemy At Closest Spawning Point`
  (bind _spawnpoints (`self.SpawnPoints`))
  (bind _outactors (`GameplayStatics.GetAllActorsOfClass` "/Game/Blueprints/Enemy_BP.Enemy_BP_C"))
  (if (< (`KismetArrayLibrary.Array_Length` _outactors) (`self.MaxEnemyCount`))
    ;[1 1 1] Spawn enemy at closest spawning point to player and make it chase player and friends
    (`KismetSystemLibrary.Delay` (`self.EnemySpawnDelay`))
    (`KismetArrayLibrary.Array_Resize` (`self.SpawnPointsDistancesToPlayer`) (`KismetArrayLibrary.Array_Length` _spawnpoints))
    (for (_array_element _array_index) _spawnpoints
      (`KismetArrayLibrary.Array_Set` (`self.SpawnPointsDistancesToPlayer`) _array_index (`KismetMathLibrary.VSize` (- (`self.K2_GetActorLocation` (`GameplayStatics.GetPlayerPawn` 0)) _array_element))))
    (bind _returnvalue (`|SpawnActorFromClass` "/Game/Blueprints/Enemy_BP.Enemy_BP_C" (`KismetMathLibrary.Conv_VectorToTransform` (`|GetArrayItem` (`self.SpawnPoints`) (`KismetMathLibrary.MinOfFloatArray` (`self.SpawnPointsDistancesToPlayer`)))) "AdjustIfPossibleButAlwaysSpawn" "OverrideRootScale" null null))
    (`/Game/Blueprints/Enemy_BP.Chase Actor` _returnvalue)))

(fn `UserConstructionScript`)