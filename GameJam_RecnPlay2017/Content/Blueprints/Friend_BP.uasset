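; Friend pawn that joins a conga-style follower line, the GameMode's TremzinhoDaAlegria array, when the player hits it.
; On its first such hit it appends itself to the array and follows the entry just before it.
; Following uses AI MoveTo, reissued after each success to keep tracking that actor.
; Each new join also calls ChaseActor on every Enemy_BP in the level so they update their chase target.
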(event `Follow Actor`
  (params (TargetActor :type "Pawn Object Reference"))
  ;[1 1 1] This friend follow Target Actor
  (`|AIMoveTo` self (0.0 0.0 0.0) TargetActor
    (:`OnSuccess`
      (`self.Follow Actor` TargetActor))))

(event `self.ReceiveHit`
  (params (MyComp :type "PrimitiveComponent Object Reference") (Other :type "Actor Object Reference") (OtherComp :type "PrimitiveComponent Object Reference") (bSelfMoved :type Boolean) (HitLocation :type "Vector Structure") (HitNormal :type "Vector Structure") (NormalImpulse :type "Vector Structure") (Hit :type "HitResult Structure (by ref)"))
  ;[1 1 1] When Player hits this friend, add this friend to Friends Array (if not already in it), and make this friend follow the second to last friend in array
  (if (== Other (`GameplayStatics.GetPlayerPawn` 0))
    (bind _asrecn_play_game_mode_bp (cast `/Game/Blueprints/RecnPlay_GameMode_BP` (`GameplayStatics.GetGameMode`)))
    (bind _tremzinhodaalegria (`/Game/Blueprints/RecnPlay_GameMode_BP.TremzinhoDaAlegria` _asrecn_play_game_mode_bp))
    (if (not (`KismetArrayLibrary.Array_Contains` _tremzinhodaalegria self))
      (`KismetArrayLibrary.Array_Add` _tremzinhodaalegria self)
      (`self.Follow Actor` (`|GetArrayItem` _tremzinhodaalegria (- (`KismetArrayLibrary.Array_LastIndex` _tremzinhodaalegria) 1)))
      ;[1 1 1] When a new friend joins the line, re-tell every enemy which target to chase
      (bind _outactors (`GameplayStatics.GetAllActorsOfClass` "/Game/Blueprints/Enemy_BP.Enemy_BP_C"))
      (for _array_element _outactors
        (`/Game/Blueprints/Enemy_BP.Chase Actor` _array_element)))))

(fn `UserConstructionScript`)