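; Enemy Blueprint that chases the last actor in the game mode's TremzinhoDaAlegria array and is meant to respawn after reaching it.
; ChaseActor uses AIMoveTo and, on success, triggers destroy-and-respawn, which calls DestroyActor before waiting on the respawn timer.
; SpawnAtRandomSpawnPoint then spawns a new Enemy_BP at a random game mode spawn point, adjusting for collisions.
; No event in this graph starts the chase itself.
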(event `Spawn At Random Spawn Point`
  (bind _asrecn_play_game_mode_bp (cast `/Game/Blueprints/RecnPlay_GameMode_BP` (`GameplayStatics.GetGameMode`)))
  (bind _spawnpoints (`/Game/Blueprints/RecnPlay_GameMode_BP.SpawnPoints` _asrecn_play_game_mode_bp))
  (`|SpawnActorFromClass` "Enemy_BP_C" (`|GetArrayItem` _spawnpoints (`KismetMathLibrary.RandomInteger` (`KismetArrayLibrary.Array_LastIndex` _spawnpoints))) "AdjustIfPossibleButAlwaysSpawn" "OverrideRootScale" null null))

(event `Chase Actor`
  (bind _asrecn_play_game_mode_bp (cast `/Game/Blueprints/RecnPlay_GameMode_BP` (`GameplayStatics.GetGameMode`)))
  (bind _tremzinhodaalegria (`/Game/Blueprints/RecnPlay_GameMode_BP.TremzinhoDaAlegria` _asrecn_play_game_mode_bp))
  (`|AIMoveTo` self (0.0 0.0 0.0) (`|GetArrayItem` _tremzinhodaalegria (`KismetArrayLibrary.Array_LastIndex` _tremzinhodaalegria))
    (:`OnSuccess`
      (`self.Destroy and Respawn`))))

(event `Destroy and Respawn`
  (`self.K2_DestroyActor`)
  (`KismetSystemLibrary.Delay` (`self.EnemyRespawnTimer`))
  (`self.Spawn At Random Spawn Point`))

(fn `UserConstructionScript`)